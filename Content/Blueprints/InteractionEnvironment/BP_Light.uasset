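; BP_Light is a toggleable point light actor driven by a BP_Button in the level.
; On BeginPlay it reads the light's initial visibility into IsLightOn, then binds to OnButtonPressed on the single BP_Button returned by GetActorOfClass.
; Each press flips the state through TurnLightOn or TurnLightOff, which set visibility and update the flag.
; Switchon and SwitchOff events set the state directly, and IsActive reports it.
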(event `self.ReceiveBeginPlay`
  (set `self.IsLightOn` (`SceneComponent.bVisible` (`self.PointLight`)))
  (bind _returnvalue (`GameplayStatics.GetActorOfClass` "/Game/Blueprints/InteractionEnvironment/BP_Button.BP_Button_C"))
  (add `/Game/Blueprints/InteractionEnvironment/BP_Button.OnButtonPressed` _returnvalue (delegate `EventOnButtonPressed`)) ; Подписка на выключатель
)

(event `EventOnButtonPressed`
  (if (`self.IsLightOn`)
    (`self.TurnLightOff`)
    (else
      (`self.TurnLightOn`))))

(event `/Game/Blueprints/Interfaces/BPI_Switchable.SwitchOn`
  (`self.TurnLightOn`))

(event `/Game/Blueprints/Interfaces/BPI_Switchable.SwitchOff`
  (`self.TurnLightOff`))

(fn `IsActive`
  (returns (IsLightOn :type Boolean))
  (return (`self.IsLightOn`)))

(fn `TurnLightOff`
  (`SceneComponent.SetVisibility` (`self.PointLight`) false false)
  (set `self.IsLightOn` false))

(fn `TurnLightOn`
  (`SceneComponent.SetVisibility` (`self.PointLight`) true false)
  (set `self.IsLightOn` true)
  (return))

(fn `UserConstructionScript`)